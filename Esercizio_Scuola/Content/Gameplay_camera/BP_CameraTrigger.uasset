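; Camera trigger zone that calls ChangeCamera with its CameraActor when the player enters the collision and with no camera on exit.
; Every tick, regardless of overlap, CameraActor rotates to face the player.
; Tick also sets the trigger actor's own location, interpolated from CameraActor's position toward the spline point closest to the player.
; Overlap events also print debug greetings.
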(event OnComponentEndOverlap(CollisionComponent)
  (params (OverlappedComponent :type Primitive%20Component%20Object%20Reference) (OtherActor :type Actor%20Object%20Reference) (OtherComp :type Primitive%20Component%20Object%20Reference) (OtherBodyIndex :type Integer))
  (if (== OtherActor (Game|GetPlayerCharacter 0))
    (Development|PrintString "Addio")
    (Default|CallChangeCamera)))

(event OnComponentBeginOverlap(CollisionComponent)
  (params (OverlappedComponent :type Primitive%20Component%20Object%20Reference) (OtherActor :type Actor%20Object%20Reference) (OtherComp :type Primitive%20Component%20Object%20Reference) (OtherBodyIndex :type Integer) (bFromSweep :type Boolean) (SweepResult :type Hit%20Result%20Structure%20%28by%20ref%29))
  (if (== OtherActor (Game|GetPlayerCharacter 0))
    (Development|PrintString "Benvenuto")
    (Default|CallChangeCamera (Variables|Default|GetCameraActor))))

(event EventBeginPlay)

(event Collision|EventActorBeginOverlap
  (params (OtherActor :type Actor%20Object%20Reference)))

(event EventTick
  (params (DeltaSeconds :type Float%20%28single-precision%29))
  (bind _cameraactor (Variables|Default|GetCameraActor))
  (bind _returnvalue (Transformation|GetActorLocation _cameraactor))
  (Transformation|SetActorRotation (Variables|Default|GetCameraActor) (Math|Rotator|MakeRotationfromAxes (- (Transformation|GetActorLocation (Game|GetPlayerCharacter 0)) _returnvalue) "0, 0, 0" "0, 0, 0"))
  (Transformation|SetActorLocation (Math|Interpolation|VInterpTo _returnvalue (Spline|FindLocationClosesttoWorldLocation (Variables|Default|GetSpline) (Transformation|GetActorLocation (Game|GetPlayerCharacter 0)) "World") (Utilities|Time|GetWorldDeltaSeconds) 1.0) false false))

(fn ConstructionScript)