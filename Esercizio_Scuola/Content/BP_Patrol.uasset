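; BP_Patrol is a patrol route that steps an index back and forth along the points of a Spline.
; IncrematePatrolling advances PatrolIndex by Direction, flipping to forward at zero and to backward when the following step would hit the last point, so that point is never reached going forward from zero.
; GetSplinePointAsWorldCoordinates returns the current point's location, in Local space despite its name.
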(event Custom|IncrematePatrolling
  (Variables|Default|SetPatrolIndex (+ (Variables|Default|GetPatrolIndex) (Variables|Default|GetDirection)))
  (if (== (+ (Variables|Default|GetPatrolIndex) (Variables|Default|GetDirection)) (- (Spline|GetNumberOfSplinePoints (Variables|Default|GetSpline)) 1))
    (Variables|Default|SetDirection -1)
    (elif (== (Variables|Default|GetPatrolIndex) 0)
      (Variables|Default|SetDirection 1))))

(fn ConstructionScript)

(fn GetSplinePointasWorldCoordinates
  (return (Spline|GetLocationatSplinePoint (Variables|Default|GetSpline) (Variables|Default|GetPatrolIndex) "Local")))