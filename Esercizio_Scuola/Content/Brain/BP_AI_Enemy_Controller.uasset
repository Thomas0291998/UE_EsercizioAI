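; Enemy AI controller that runs BT_Enemy on possess and sets the blackboard AiState to idle after a short delay.
; On perception updates, a CanSense helper matches each actor's last stimuli by sense class, and a failed sight check returns the state to idle.
; Hearing checks and both handler functions are stubs.
; SetStateAsAttacking, which targets the player character, is defined but never called here.
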(event OnPerceptionUpdated(AIPerception)
  (params (UpdatedActors :type Array%20of%20Actor%20Object%20References))
  (for _array_element UpdatedActors
    (Utilities|FlowControl|Sequence
      (:then_0
        (bind _successfully_sensed (CallFunction|CanSense _array_element "NewEnumerator1"))
        (if (not _successfully_sensed)
          (CallFunction|SetStateasIdle)))
      (:then_1
        (CallFunction|CanSense _array_element "NewEnumerator0")
        (if true
          _)))))

(event EventPossess
  (params (PossessedPawn :type Pawn%20Object%20Reference))
  (AI|RunBehaviorTree "/Game/Brain/BT_Enemy.BT_Enemy")
  (Utilities|FlowControl|Delay 0.2)
  (CallFunction|SetStateasIdle))

(fn ConstructionScript)

(fn SetStateasIdle
  (AI|Components|Blackboard|SetValueasEnum (Variables|Default|GetBlackboard) (Utilities|Name|MakeLiteralName "AiState") (Utilities|Enum|LiteralenumAiState "NewEnumerator1")))

(fn SetStateasAttacking
  (AI|Components|Blackboard|SetValueasObject (Variables|Default|GetBlackboard) (Utilities|Name|MakeLiteralName "Target") (Game|GetPlayerCharacter 0))
  (AI|Components|Blackboard|SetValueasEnum (Variables|Default|GetBlackboard) (Utilities|Name|MakeLiteralName "AiState") (Utilities|Enum|LiteralenumAiState "NewEnumerator2")))

(fn CanSense
  (params (Actor :type Actor%20Object%20Reference) (Index :type E_Sense%20Enum :default "NewEnumerator0"))
  (bind _info (Class|AIPerceptionComponent|GetActorsPerception (Variables|Default|GetAIPerception) Actor))
  (for _array_element (.LastSensedStimuli (Utilities|Struct|BreakActorPerceptionBlueprintInfo _info))
    (bind _returnvalue (Class|AIPerceptionSystem|GetSenseClassforStimulus _array_element))
    (if (== _returnvalue (Utilities|Select :Index Index :NewEnumerator0 0 :NewEnumerator1 0))
      (return (.StimulusLocation (Utilities|Struct|BreakAIStimulus _array_element)) (.bSuccessfullySensed (Utilities|Struct|BreakAIStimulus _array_element))))))

(fn HandleHearing)

(fn HandleSight)